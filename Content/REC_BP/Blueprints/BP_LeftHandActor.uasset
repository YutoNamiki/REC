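; BP_LeftHandActor is a left-hand actor that casts a visible pointing ray from its DirectionArrow component.
; Every Tick runs an object line trace 1000 units along the arrow's forward vector against WorldStatic, redrawing the debug line each frame.
; The hit result is unused, and no other event or construction logic is implemented.
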(event `self.ReceiveTick`
  (params (DeltaSeconds :type "Float (single-precision)"))
  (bind _directionarrow (`self.DirectionArrow`))
  (bind _returnvalue (`SceneComponent.K2_GetComponentLocation` _directionarrow))
  (`parent.ReceiveTick` DeltaSeconds)
  (`KismetSystemLibrary.LineTraceSingleForObjects` :`Start` _returnvalue :`End` (+ _returnvalue (* (`SceneComponent.GetForwardVector` _directionarrow) 1000.0)) :`ObjectTypes` (`|MakeArray` "ObjectTypeQuery1" :!type "EObjectTypeQuery Enum") :`DrawDebugType` "ForDuration" :`DrawTime` 0.0))

(fn `UserConstructionScript`
  (`parent.UserConstructionScript`))